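; BP_Naration is a narration Blueprint that plays a fixed sequence of six voice dialogue lines, starting on BeginPlay.
; Each line is spawned as non-spatial 2D dialogue using a shared Speaker context.
; Every spawned audio component binds its OnAudioFinished event to a custom event that spawns the next line, forming a hard-coded chain that ends after the sixth.
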(event `self.ReceiveBeginPlay`
  (bind _returnvalue (`GameplayStatics.SpawnDialogue2D` (`self.Dialogue`) (`self.Speaker`)))
  (add `AudioComponent.OnAudioFinished` _returnvalue (delegate `AudioFinished`)))

(event `AudioFinished`
  (bind _returnvalue (`GameplayStatics.SpawnDialogue2D` (`self.Dialogue_2`) (`self.Speaker`)))
  (add `AudioComponent.OnAudioFinished` _returnvalue (delegate `CustomEvent_0`)))

(event `CustomEvent_0`
  (bind _returnvalue (`GameplayStatics.SpawnDialogue2D` (`self.Dialogue_3`) (`self.Speaker`)))
  (add `AudioComponent.OnAudioFinished` _returnvalue (delegate `CustomEvent`)))

(event `CustomEvent`
  (bind _returnvalue (`GameplayStatics.SpawnDialogue2D` (`self.Dialogue_4`) (`self.Speaker`)))
  (add `AudioComponent.OnAudioFinished` _returnvalue (delegate `CustomEvent_1`)))

(event `CustomEvent_1`
  (bind _returnvalue (`GameplayStatics.SpawnDialogue2D` (`self.Dialogue_5`) (`self.Speaker`)))
  (add `AudioComponent.OnAudioFinished` _returnvalue (delegate `CustomEvent_2`)))

(event `CustomEvent_2`
  (`GameplayStatics.SpawnDialogue2D` (`self.Dialogue_6`) (`self.Speaker`)))

(fn `UserConstructionScript`)