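; Player character Blueprint that handles item interaction, a widget-based inventory and a pause menu.
; Capsule overlap caches the item, whose interaction widget follows the Interaction input, while I and Escape flip-flop the menus.
; PickUpItem stacks onto matching inventory widgets or adds new ones, and DropItem spawns the item ahead and pushes it away.
; Items live only as InventoryWBP children, and that widget is recreated each time I opens it.
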(event `Key|I`
  (params (Key :type "Key Structure"))
  (bind _returnvalue (`GameplayStatics.GetPlayerController` 0))
  (bind _returnvalue_2 (`GameplayStatics.GetPlayerController` 0))
  (:`Pressed`
    (`/Engine/EditorBlueprintResources/StandardMacros.FlipFlop`
      (:`A`
        (bind _returnvalue_3 (`|CreateWidget` "/Game/CYS/CYS_BluePrints/CYS_WBP_Inventory.CYS_WBP_Inventory_C"))
        (bind _output_get (set `self.inventory_WBP` _returnvalue_3))
        (`UserWidget.AddToViewport` _output_get 0)
        (`WidgetBlueprintLibrary.SetInputMode_GameAndUIEx` _returnvalue_2 null)
        (set `PlayerController.bShowMouseCursor` true _returnvalue_2))
      (:`B`
        (set `PlayerController.bShowMouseCursor` false _returnvalue)
        (`Widget.SetVisibility` _returnvalue_3 "Hidden")
        (`WidgetBlueprintLibrary.SetInputMode_GameOnly` _returnvalue)))))

(event `InputAction|Interaction`
  (params (Key :type "Key Structure"))
  (bind _as_bp_test_item_parants (`self.As BP Test Item Parants`))
  ;[1 0.6742 0.2633 1 48] 상호작용
  (:`Pressed`
    (bind _asbp_test_item_parants (cast `/Game/CYS/CYS_BluePrints/BP_TestItemParants` _as_bp_test_item_parants))
    (set `/Game/CYS/CYS_BluePrints/WBP_Interaction.isPressed` true (`/Game/CYS/CYS_BluePrints/BP_TestItemParants.interactionWidget` _asbp_test_item_parants)))
  (:`Released`
    (bind _asbp_test_item_parants_2 (cast `/Game/CYS/CYS_BluePrints/BP_TestItemParants` _as_bp_test_item_parants))
    (set `/Game/CYS/CYS_BluePrints/WBP_Interaction.isPressed` false (`/Game/CYS/CYS_BluePrints/BP_TestItemParants.interactionWidget` _asbp_test_item_parants_2))))

(event `Key|Escape` :paused true
  (params (Key :type "Key Structure"))
  (bind _returnvalue (`GameplayStatics.GetPlayerController` 0))
  (:`Pressed`
    (`/Engine/EditorBlueprintResources/StandardMacros.FlipFlop`
      (:`A`
        (bind _returnvalue_2 (`|CreateWidget` "/Game/CYS/CYS_BluePrints/WBP_PauseMenu.WBP_PauseMenu_C"))
        (`UserWidget.AddToViewport` _returnvalue_2 0))
      (:`B`
        (set `PlayerController.bShowMouseCursor` false _returnvalue)
        (`Widget.RemoveFromParent` _returnvalue_2)
        (`GameplayStatics.SetGamePaused` false)
        (`WidgetBlueprintLibrary.SetInputMode_GameOnly` _returnvalue)))))

(event `self.CapsuleComponent.OnComponentBeginOverlap`
  (params (OverlappedComponent :type "PrimitiveComponent Object Reference") (OtherActor :type "Actor Object Reference") (OtherComp :type "PrimitiveComponent Object Reference") (OtherBodyIndex :type Integer) (bFromSweep :type Boolean) (SweepResult :type "HitResult Structure (by ref)"))
  ;[1 0.6742 0.2633 1 48] 상호작용
  (bind _asbp_test_item_parants (cast `/Game/CYS/CYS_BluePrints/BP_TestItemParants` OtherActor))
  (set `self.As BP Test Item Parants` _asbp_test_item_parants))

(event `/Game/CYS/CYS_BluePrints/BPI_PickupItem.PickUpItem`
  (params (itemClass :type "Actor Class Reference") (itemIcon :type "Texture2D Object Reference") (stackAmount :type Integer))
  (`self.AddItemInventory` itemClass itemIcon stackAmount))

(event `/Game/CYS/CYS_BluePrints/BPI_PickupItem.DropItem`
  (params (itemClass :type "Actor Class Reference"))
  (bind _returnvalue (`|SpawnActorFromClass` itemClass (`KismetMathLibrary.MakeTransform` (+ (`self.K2_GetActorLocation`) (* (`KismetMathLibrary.GetForwardVector` (`self.K2_GetActorRotation`)) 150.0))) "AlwaysSpawn" "OverrideRootScale" null null))
  (message `/Game/CYS/CYS_BluePrints/BPI_PickupItem.PushPickupItemAway` _returnvalue))

(fn `AddItemInventory`
  (params (itemClass :type "Actor Class Reference") (Texture :type "Texture2D Object Reference") (MaxStack :type Integer))
  (if (> MaxStack 1)
    ;[1 1 1] 용도 체크
    (for _array_element (`PanelWidget.GetAllChildren` (`/Game/CYS/CYS_BluePrints/CYS_WBP_Inventory.InventoryBox` (`self.inventory_WBP`)))
      (bind (_itemclass _currentstack _maxstack) (message `/Game/CYS/CYS_BluePrints/BPI_PickupItem.PickUpItemData` _array_element))
      (if (== _itemclass itemClass)
        (if (<= (+ _currentstack 1) _maxstack)
          (message `/Game/CYS/CYS_BluePrints/BPI_PickupItem.PickupItemStack` _array_element)
          (set `self.isPickupItem` true)
          (break))))
    (if (not (`self.isPickupItem`))
      (bind _returnvalue (`|CreateWidget` "/Game/CYS/CYS_BluePrints/WBP_PickUpItem.WBP_PickUpItem_C" :!label _label))
      (set `/Game/CYS/CYS_BluePrints/WBP_PickUpItem.itemClass` itemClass _returnvalue)
      (`Image.SetBrush` (`/Game/CYS/CYS_BluePrints/WBP_PickUpItem.ItemIcon` _returnvalue) (`WidgetBlueprintLibrary.MakeBrushFromTexture` Texture 100 100))
      (set `/Game/CYS/CYS_BluePrints/WBP_PickUpItem.maxStack` MaxStack _returnvalue)
      (`WrapBox.AddChildToWrapBox` (`/Game/CYS/CYS_BluePrints/CYS_WBP_Inventory.InventoryBox` (`self.inventory_WBP`)) _returnvalue))
    (else
      (goto _label))))

(fn `PickUpItemData`
  (returns (itemClass :type "Actor Class Reference") (currentStack :type Integer) (maxStack :type Integer))
  (return null 0 0))

(fn `UserConstructionScript`)