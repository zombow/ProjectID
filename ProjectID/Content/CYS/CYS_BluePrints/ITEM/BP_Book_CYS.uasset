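; BP_Book_CYS is a book item that shows an interaction prompt while a CYS_TestCharacter is inside its overlap sphere.
; An interaction widget created at BeginPlay joins the viewport on entry, when the book also stores itself in ItemParants, and leaves on exit.
; The overlap also toggles the floating text and actor tick, which rotates the text toward the player.
; The interaction action itself is not handled in this graph.
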(event `self.ReceiveBeginPlay`
  (bind _returnvalue (`|CreateWidget` "/Game/CYS/CYS_BluePrints/WBP_Interaction.WBP_Interaction_C" (`GameplayStatics.GetPlayerController` 0)))
  (set `self.interactionWidget` _returnvalue))

(event `self.Sphere.OnComponentBeginOverlap`
  (params (OverlappedComponent :type "PrimitiveComponent Object Reference") (OtherActor :type "Actor Object Reference") (OtherComp :type "PrimitiveComponent Object Reference") (OtherBodyIndex :type Integer) (bFromSweep :type Boolean) (SweepResult :type "HitResult Structure (by ref)"))
  (cast `/Game/CYS/CYS_BluePrints/ITEM/CYS_TestCharacter` OtherActor)
  (set `self.itemParants` self)
  (set `self.overlapitem` true)
  (`UserWidget.AddToViewport` (`self.interactionWidget`) 0)
  (`SceneComponent.SetVisibility` (`self.TextRender`) true true)
  (`self.SetActorTickEnabled` true))

(event `self.Sphere.OnComponentEndOverlap`
  (params (OverlappedComponent :type "PrimitiveComponent Object Reference") (OtherActor :type "Actor Object Reference") (OtherComp :type "PrimitiveComponent Object Reference") (OtherBodyIndex :type Integer))
  (cast `/Game/CYS/CYS_BluePrints/ITEM/CYS_TestCharacter` OtherActor)
  (set `self.overlapitem` false)
  (`Widget.RemoveFromParent` (`self.interactionWidget`))
  (`SceneComponent.SetVisibility` (`self.TextRender`) false true)
  (`self.SetActorTickEnabled` false)
  (set `self.overlapitem` false))

(event `self.ReceiveTick`
  (params (DeltaSeconds :type "Float (single-precision)"))
  (if (`self.overlapitem`)
    (`SceneComponent.K2_SetWorldRotation` (`self.TextRender`) (`KismetMathLibrary.FindLookAtRotation` (`SceneComponent.K2_GetComponentLocation` (`self.TextRender`)) (`self.K2_GetActorLocation` (`GameplayStatics.GetPlayerCharacter` 0))) false false)))

(fn `UserConstructionScript`)