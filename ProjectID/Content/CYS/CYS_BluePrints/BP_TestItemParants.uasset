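; BP_TestItemParants is a test parent actor for pickup items that shows an interaction prompt when the player character is nearby.
; Sphere overlap toggles the interaction widget, a text label and actor tick, which turns the label toward the player.
; PushPickupItemAway impulses the mesh along the camera's forward direction.
; The interface-based pickup-and-destroy logic is disconnected, and PickUpItemData returns only zero stack values.
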(event `self.ReceiveBeginPlay`
  (bind _returnvalue (`|CreateWidget` "/Game/CYS/CYS_BluePrints/WBP_Interaction.WBP_Interaction_C" (`GameplayStatics.GetPlayerController` 0)))
  (set `self.interactionWidget` _returnvalue))

(event `self.Sphere.OnComponentBeginOverlap`
  (params (OverlappedComponent :type "PrimitiveComponent Object Reference") (OtherActor :type "Actor Object Reference") (OtherComp :type "PrimitiveComponent Object Reference") (OtherBodyIndex :type Integer) (bFromSweep :type Boolean) (SweepResult :type "HitResult Structure (by ref)"))
  (cast `/Game/CYS/CYS_BluePrints/BP_CYS_Chracter` OtherActor)
  (set `self.itemParants` self)
  (set `self.overlapitem` true)
  (`UserWidget.AddToViewport` (`self.interactionWidget`) 0)
  (`SceneComponent.SetVisibility` (`self.TextRender`) true true)
  (`self.SetActorTickEnabled` true))

(event `self.Sphere.OnComponentEndOverlap`
  (params (OverlappedComponent :type "PrimitiveComponent Object Reference") (OtherActor :type "Actor Object Reference") (OtherComp :type "PrimitiveComponent Object Reference") (OtherBodyIndex :type Integer))
  (cast `/Game/CYS/CYS_BluePrints/BP_CYS_Chracter` OtherActor)
  (set `self.overlapitem` false)
  (`Widget.RemoveFromParent` (`self.interactionWidget`))
  (`SceneComponent.SetVisibility` (`self.TextRender`) false true)
  (`self.SetActorTickEnabled` false)
  (set `self.overlapitem` false))

(event `self.ReceiveTick`
  (params (DeltaSeconds :type "Float (single-precision)"))
  (if (`self.overlapitem`)
    (`SceneComponent.K2_SetWorldRotation` (`self.TextRender`) (`KismetMathLibrary.FindLookAtRotation` (`SceneComponent.K2_GetComponentLocation` (`self.TextRender`)) (`self.K2_GetActorLocation` (`GameplayStatics.GetPlayerCharacter` 0))) false false)))

(event `/Game/CYS/CYS_BluePrints/BPI_PickupItem.PushPickupItemAway`
  (bind _returnvalue (`KismetMathLibrary.GetForwardVector` (`PlayerCameraManager.GetCameraRotation` (`GameplayStatics.GetPlayerCameraManager` 0))))
  (`PrimitiveComponent.AddVelocityChangeImpulseAtLocation` (`self.StaticMesh`) (* _returnvalue 250.0) (+ (`self.K2_GetActorLocation`) (* _returnvalue (15.0 0.0 0.0))) "None"))

(fn `PickUpItemData`
  (returns (itemClass :type "Actor Class Reference") (currentStack :type Integer) (maxStack :type Integer))
  (return null 0 0))

(fn `UserConstructionScript`)