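; Frame puzzle Blueprint that provides the response when the puzzle is solved, revealing hidden meshes and moving two curtains toward open.
; The FramePuzzleSolved event shows the StaticMesh and Plane components, then calls CurtainOpen with world delta seconds as both alphas.
; CurtainOpen lerps each referenced curtain actor's X scale toward mirrored targets, one step per call.
; Tick is empty, so any gradual opening depends on the event being fired repeatedly.
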(event `self.ReceiveTick`
  (params (DeltaSeconds :type "Float (single-precision)")))

(event `/Game/DY/Blueprints/BPI_ItemInteraction.FramePuzzleSolved`
  (bind _returnvalue (`GameplayStatics.GetWorldDeltaSeconds`))
  (`SceneComponent.SetVisibility` (`self.StaticMesh`) true false)
  (`SceneComponent.SetVisibility` (`self.Plane`) true false)
  (`self.CurtainOpen` _returnvalue _returnvalue))

(fn `CurtainOpen`
  (params (Alpha :type "Float (double-precision)") (Alpha2 :type "Float (double-precision)"))
  (bind _leftcurtain (`self.leftCurtain`))
  (bind _rightcurtain (`self.rightCurtain`))
  (bind (_returnvalue_x _returnvalue_y _returnvalue_z) (`KismetMathLibrary.BreakVector` (`self.GetActorScale3D` _rightcurtain)))
  (bind (_returnvalue_x_2 _returnvalue_y_2 _returnvalue_z_2) (`KismetMathLibrary.BreakVector` (`self.GetActorScale3D` _leftcurtain)))
  (`self.SetActorScale3D` _leftcurtain (`KismetMathLibrary.MakeVector` (`KismetMathLibrary.Lerp` _returnvalue_x_2 1.0 Alpha) _returnvalue_y_2 _returnvalue_z_2))
  (`self.SetActorScale3D` _rightcurtain (`KismetMathLibrary.MakeVector` (`KismetMathLibrary.Lerp` _returnvalue_x -1.0 Alpha2) _returnvalue_y _returnvalue_z)))

(fn `UserConstructionScript`)