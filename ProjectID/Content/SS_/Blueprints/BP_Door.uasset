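; Door actor that serves as either a small-room door or a restroom door, swinging slightly open, further open, or closed.
; ProccedInteraction maps an index to state flags, switching to restroom flags once the small room is solved.
; Tick picks door functions by IsSmallRoom and acts on those flags.
; Restroom opening eases yaw by delta-time Lerp, while closing, run only for the small room, snaps instantly.
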(event `self.ReceiveBeginPlay`)

(event `self.ReceiveTick`
  (params (DeltaSeconds :type "Float (single-precision)"))
  (if (`self.bIsSmallRoom`)
    (`|ExecutionSequence`
      (:`then_0`
        (`self.DoorSlightlyOpen`))
      (:`then_1`
        (`self.DoorOpen`))
      (:`then_2`
        (`self.DoorClose`)))
    (else
      (`|ExecutionSequence`
        (:`then_0`
          (`self.RestRoomDoorSlightlyOpen`))
        (:`then_1`
          (`self.RestRoomDoorOpen`))))))

(event `LevelInterface.ProccedInteraction`
  (params (indexNum :type Integer))
  (if (`self.bIsSmallRoomSolved`)
    (switch `int` indexNum
      (:`0`
        (set `self.bIsRestRoomOpen` true))
      (:`1`
        (set `self.bIsRestRoomOpenInteraction` true))
      (:`2`
        (set `self.bCloseInteraction` true)))
    (else
      (switch `int` indexNum
        (:`0`
          (set `self.bIsOpen` true))
        (:`1`
          (set `self.bIsOpenInteraction` true))
        (:`2`
          (set `self.bCloseInteraction` true))
        (:`3`
          (`self.SmallRoomSolved`))))))

(fn `DoorClose`
  (bind (_returnvalue_roll _returnvalue_pitch _returnvalue_yaw) (`KismetMathLibrary.BreakRotator` (`self.K2_GetActorRotation`)))
  (if (`self.bCloseInteraction`)
    (`self.K2_SetActorRotation` (`KismetMathLibrary.MakeRotator` 0.0 0.0 (`KismetMathLibrary.Lerp` _returnvalue_yaw 179.999999 1.0)))
    (set `self.bCloseInteraction` false)))

(fn `RestRoomDoorOpen`
  (bind (_returnvalue_roll _returnvalue_pitch _returnvalue_yaw) (`KismetMathLibrary.BreakRotator` (`self.K2_GetActorRotation`)))
  (if (`self.bIsRestRoomOpenInteraction`)
    (`self.K2_SetActorRotation` (`KismetMathLibrary.MakeRotator` 0.0 0.0 (`KismetMathLibrary.Lerp` 70.0 _returnvalue_yaw (- 1.0 (`GameplayStatics.GetWorldDeltaSeconds`)))))))

(fn `RestRoomDoorSlightlyOpen`
  (bind (_returnvalue_roll _returnvalue_pitch _returnvalue_yaw) (`KismetMathLibrary.BreakRotator` (`self.K2_GetActorRotation`)))
  (if (`self.bIsRestRoomOpen`)
    (`self.K2_SetActorRotation` (`KismetMathLibrary.MakeRotator` 0.0 0.0 (`KismetMathLibrary.Lerp` 159.999999 _returnvalue_yaw (- 1.0 (`GameplayStatics.GetWorldDeltaSeconds`)))))))

(fn `SmallRoomSolved`
  (set `self.openAngle` 0.0)
  (set `self.bIsSmallRoomSolved` true))

(fn `UserConstructionScript`)