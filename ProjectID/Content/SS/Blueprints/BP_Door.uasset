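; Door actor that serves as either a small-room door or a restroom door, chosen by IsSmallRoom.
; ProccedInteraction maps an index to open or close flags, switching to restroom flags once the small room is solved.
; Tick polls those flags, rotating the door by stepped yaw or per-frame lerp, while closing snaps shut.
; A test character entering the capsule trigger also sets the restroom full-open flag, effective once slightly open.
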(event `self.ReceiveBeginPlay`)

(event `self.ReceiveTick`
  (params (DeltaSeconds :type "Float (single-precision)"))
  (if (`self.bIsSmallRoom`)
    (`|ExecutionSequence`
      (:`then_0`
        (`self.DoorSlightlyOpentest`))
      (:`then_1`
        (`self.DoorOpen`))
      (:`then_2`
        (`self.DoorClose`)))
    (else
      (`|ExecutionSequence`
        (:`then_0`
          (`self.RestRoomDoorSlightlyOpen`))
        (:`then_1`
          (`self.RestRoomDoorOpen`))))))

(event `LevelInterface.ProccedInteraction`
  (params (indexNum :type Integer))
  (if (`self.bIsSmallRoomSolved`)
    (switch `int` indexNum
      (:`0`
        (set `self.bIsRestRoomOpen` true))
      (:`1`
        (set `self.bIsRestRoomOpenInteraction` true))
      (:`2`
        (set `self.bCloseInteraction` true)))
    (else
      (`KismetSystemLibrary.PrintText` "Hello" true true (struct :`G` 0.66 :`B` 1.0 :`A` 1.0) 20.0)
      (switch `int` indexNum
        (:`0`
          (set `self.bIsOpen` true))
        (:`1`
          (set `self.bIsOpenInteraction` true))
        (:`2`
          (set `self.bCloseInteraction` true))
        (:`3`
          (`self.SmallRoomSolved`))))))

(event `self.doorCapsulCollComp.OnComponentBeginOverlap`
  (params (OverlappedComponent :type "PrimitiveComponent Object Reference") (OtherActor :type "Actor Object Reference") (OtherComp :type "PrimitiveComponent Object Reference") (OtherBodyIndex :type Integer) (bFromSweep :type Boolean) (SweepResult :type "HitResult Structure (by ref)"))
  (cast `/Game/AYU/AYU_Blueprints/AYU_TestCharacter` OtherActor)
  (set `self.bIsRestRoomOpenInteraction` true))

(fn `DoorClose`
  (bind (_returnvalue_roll _returnvalue_pitch _returnvalue_yaw) (`KismetMathLibrary.BreakRotator` (`self.K2_GetActorRotation`)))
  (if (`self.bCloseInteraction`)
    (`self.K2_SetActorRotation` (`KismetMathLibrary.MakeRotator` 0.0 0.0 (`KismetMathLibrary.Lerp` _returnvalue_yaw 179.999999 1.0)))
    (set `self.bCloseInteraction` false)))

(fn `DoorSlightlyOpentest`
  (if (`self.bIsOpen`)
    (if (< (`self.openAngle`) 20.0)
      (`self.K2_AddActorWorldRotation` (struct :`Yaw` 1.0))
      (`/Engine/EditorBlueprintResources/StandardMacros.IncrementFloat` (`self.openAngle`)))))

(fn `RestRoomDoorOpen`
  (bind (_returnvalue_roll _returnvalue_pitch _returnvalue_yaw) (`KismetMathLibrary.BreakRotator` (`self.K2_GetActorRotation`)))
  (if (`self.bIsRestRoomOpen`)
    (if (`self.bIsRestRoomOpenInteraction`)
      (`self.K2_SetActorRotation` (`KismetMathLibrary.MakeRotator` 0.0 0.0 (`KismetMathLibrary.Lerp` _returnvalue_yaw 70.0 0.1))))))

(fn `RestRoomDoorSlightlyOpen`
  (bind (_returnvalue_roll _returnvalue_pitch _returnvalue_yaw) (`KismetMathLibrary.BreakRotator` (`self.K2_GetActorRotation`)))
  (if (`self.bIsRestRoomOpen`)
    (`self.K2_SetActorRotation` (`KismetMathLibrary.MakeRotator` 0.0 0.0 (`KismetMathLibrary.Lerp` _returnvalue_yaw 159.999999 0.1)))))

(fn `SmallRoomSolved`
  (set `self.openAngle` 0.0)
  (set `self.bIsSmallRoomSolved` true))

(fn `UserConstructionScript`)