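; BP_Trigger is a one-shot overlap trigger that fires an event on the world light controller and a door when the test character enters it.
; BeginPlay looks up the BP_WorldLightCtrl and BP_Door instances by class, so it targets a single actor of each.
; On overlap by AYU_TestCharacter, it prints the actor's name, sends each target its own numbered interaction message, then sets ISEventEnd to block repeats.
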(event `self.ReceiveBeginPlay`
  (bind _returnvalue (`GameplayStatics.GetActorOfClass` "/Game/SS/Blueprints/BP_WorldLightCtrl.BP_WorldLightCtrl_C"))
  (bind _returnvalue_2 (`GameplayStatics.GetActorOfClass` "/Game/SS/Blueprints/BP_Door.BP_Door_C")))

(event `self.ReceiveActorBeginOverlap`
  (params (OtherActor :type "Actor Object Reference"))
  (if (not (`self.bISEventEnd`))
    (cast `/Game/AYU/AYU_Blueprints/AYU_TestCharacter` OtherActor)
    (`KismetSystemLibrary.PrintString` (`KismetSystemLibrary.GetDisplayName` OtherActor))
    (message `LevelInterface.ProccedInteraction` (stale `self.ReceiveBeginPlay` _returnvalue) 3)
    (message `LevelInterface.ProccedInteraction` (stale `self.ReceiveBeginPlay` _returnvalue_2) 2)
    (set `self.bISEventEnd` true)))

(fn `UserConstructionScript`)