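; World light controller that changes main-room and small-room lighting in response to indexed interaction events.
; ProccedInteraction switches on the index to light candles, turn small-room lights on or off, or tint room lights red.
; The main-room tint saves each light's original color in an array so a later interaction can restore it.
; A book check reveals the small-room candle with a sound when four tagged BP_Book actors are checked.
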(event `self.ReceiveBeginPlay`
  (bind _outactors (`GameplayStatics.GetAllActorsOfClassWithTag` "/Game/DY/Blueprints/BP_Book.BP_Book_C" "Book"))
  (set `self.BookList` _outactors))

(event `self.ProccedInteraction`
  (params (indexNum :type Integer))
  (switch `int` indexNum
    (:`0`
      (`self.BookCheckCheck`))
    (:`1`
      (`self.CandleLightOn` 0)
      (`GameplayStatics.PlaySoundAtLocation` "/Game/SS/Sound/CandleLightOn.CandleLightOn" (`self.K2_GetActorLocation` (`self.candleLight`)) (struct) 1.0 1.0 0.0 "/Game/SS/Sound/SA_clock.SA_clock" null null null))
    (:`2`
      (`|ExecutionSequence`
        (:`then_0`
          (`self.AmbientLightChange`))
        (:`then_1`
          (`self.smallRoomSpotLightOn` 0))))
    (:`3`
      (`|ExecutionSequence`
        (:`then_0`
          (`self.AmbientLightRecover`))
        (:`then_1`
          (`self.smallRoomLightOff` 0))))
    (:`4`
      (`|ExecutionSequence`
        (:`then_0`
          (`self.AmbientLightChange`))
        (:`then_1`
          (`self.SmallRoomAmbientLightChange`))))))

(fn `AmbientLightChange`
  (for _array_element (`self.MainRoomLight`)
    (bind _lightcomponent (`Light.LightComponent` _array_element))
    (`KismetArrayLibrary.Array_Add` (`self.MainRoomLightColor`) (`LightComponentBase.GetLightColor` _lightcomponent))
    (`LightComponent.SetLightColor` _lightcomponent (struct :`R` 0.466 :`G` 0.055823 :`B` 0.055823 :`A` 1.0) true)))

(fn `AmbientLightRecover`
  (for (_array_element _array_index) (`self.MainRoomLight`)
    (`LightComponent.SetLightColor` (`Light.LightComponent` _array_element) (`|GetArrayItem` (`self.MainRoomLightColor`) _array_index) true)))

(fn `BookCheckCheck`
  (bind _smallroomcandlelight (`self.SmallRoomCandleLight`))
  (set `self.CheckedBookNum` 0)
  (for _array_element (`self.BookList`)
    (if (`/Game/DY/Blueprints/BP_Book.bIsChecked` _array_element)
      (`/Engine/EditorBlueprintResources/StandardMacros.IncrementInt` (`self.CheckedBookNum`))))
  (if (== (`self.CheckedBookNum`) 4)
    (`SceneComponent.SetVisibility` (`Actor.RootComponent` _smallroomcandlelight) true false)
    (`GameplayStatics.PlaySoundAtLocation` "/Game/SS/Sound/CandleLightOn.CandleLightOn" (`self.K2_GetActorLocation` _smallroomcandlelight) (struct) 1.0 1.0 0.0 "/Game/SS/Sound/SA_clock.SA_clock" null null null)))

(fn `SmallRoomAmbientLightChange`
  (for _array_element (`self.SmallRoomLight`)
    (`LightComponent.SetLightColor` (`Light.LightComponent` _array_element) (struct :`R` 0.466 :`G` 0.055823 :`B` 0.055823 :`A` 1.0) true)))

(fn `UserConstructionScript`)