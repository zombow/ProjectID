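; Rest room event controller that reveals decals and triggers a scripted sequence around the secret door.
; Tick progressively reveals rest room decals by index, routing even counts through a short Delay, independent of the overlap.
; Player overlap reveals main room and mirror decals, flags the bloody-handprint secret door as rest-room-cleared, and stops Shot03.
; A DoOnce then plays Shot04, followed after a delay by Shot05 and the secret door spotlight.
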(event `self.ReceiveBeginPlay`
  (bind _returnvalue (`GameplayStatics.GetActorOfClass` "/Game/DY/Blueprints/SecretDoor_HandBlood_Blueprint.SecretDoor_HandBlood_Blueprint_C"))
  (set `self.SecretDoorHand` _returnvalue))

(event `self.ReceiveActorBeginOverlap`
  (params (OtherActor :type "Actor Object Reference"))
  (cast `/Game/AYU/AYU_Blueprints/AYU_TestCharacter` OtherActor)
  (for _array_element (`self.MainRoomdecalList`)
    (`SceneComponent.SetVisibility` (`Actor.RootComponent` _array_element) true false))
  (for _array_element_2 (`self.MirrorDecal`)
    (`SceneComponent.SetVisibility` (`Actor.RootComponent` _array_element_2) true false))
  (set `/Game/DY/Blueprints/SecretDoor_HandBlood_Blueprint.RestRoomClear` true (`self.SecretDoorHand`))
  (`MovieSceneSequencePlayer.Stop` (`LevelSequenceActor.SequencePlayer` (`self.shot03`)))
  (`/Engine/EditorBlueprintResources/StandardMacros.DoOnce` false
    (:`Completed`
      (`MovieSceneSequencePlayer.Play` (`LevelSequenceActor.SequencePlayer` (`self.shot04`)))
      (`KismetSystemLibrary.Delay` 3.3)
      (`MovieSceneSequencePlayer.Play` (`LevelSequenceActor.SequencePlayer` (`self.shot05`)))
      (`SceneComponent.SetVisibility` (`SpotLight.SpotLightComponent` (`self.secretDoorLight`)) true false))))

(event `self.ReceiveTick`
  (params (DeltaSeconds :type "Float (single-precision)"))
  (bind _delaycount (`self.delayCount`))
  (if (not (> _delaycount (`KismetArrayLibrary.Array_Length` (`self.RestRoomdecalList`))))
    (if (== (mod _delaycount 2.0) 0.0)
      (`KismetSystemLibrary.Delay` 0.5))
    (`SceneComponent.SetVisibility` (`Actor.RootComponent` (`|GetArrayItem` (`self.RestRoomdecalList`) (`KismetMathLibrary.FTrunc` _delaycount))) true false)
    (`/Engine/EditorBlueprintResources/StandardMacros.IncrementFloat` (`self.delayCount`))))

(fn `UserConstructionScript`)