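; BP_Weapon is a weapon prop that shows an interaction prompt while overlapped.
; BeginPlay creates pickup and interaction widgets, adds only the latter to the viewport collapsed, sets the prop name and pickup sound, and caches the player character's camera.
; Overlap events toggle the prompt, text render, static mesh and actor tick.
; While overlapped, Tick rotates the text toward the camera.
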(event `self.ReceiveBeginPlay`
  (`|ExecutionSequence`
    (:`then_0`
      (bind _returnvalue (`|CreateWidget` "/Game/CYS/CYS_BluePrints/WBP_PickUpItem_2.WBP_PickUpItem_2_C"))
      (set `self.w_Pickupitem` _returnvalue))
    (:`then_1`
      (bind _returnvalue_2 (`|CreateWidget` "/Game/CYS/CYS_BluePrints/WBP_Interaction.WBP_Interaction_C"))
      (bind _output_get (set `self.interActionUI` _returnvalue_2))
      (`UserWidget.AddToViewport` _output_get 0)
      (`Widget.SetVisibility` _output_get "Collapsed"))
    (:`then_2`
      (set `self.propsName` "Weapon"))
    (:`then_3`
      (bind _asayu_test_character (cast `/Game/AYU/AYU_Blueprints/AYU_TestCharacter` (`GameplayStatics.GetPlayerCharacter` 0)))
      (set `self.My Camera Comp` (`TestCharacter.myCameraComp` _asayu_test_character)))
    (:`then_4`
      (set `self.pickSound` "/Game/CYS/CYS_Sound/딸깍.딸깍"))))

(event `/Game/DY/Blueprints/BPI_ItemInteraction.OverlapPropsBegin`
  (set `self.overlapitem` true)
  (`Widget.SetVisibility` (`self.interActionUI`) "HitTestInvisible")
  (`SceneComponent.SetVisibility` (`self.TextRender`) true true)
  (`SceneComponent.SetHiddenInGame` (`self.StaticMesh`) false true)
  (`self.SetActorTickEnabled` true))

(event `/Game/DY/Blueprints/BPI_ItemInteraction.OverlapPropsEnd`
  (set `self.overlapitem` false)
  (`Widget.SetVisibility` (`self.interActionUI`) "Hidden")
  (`SceneComponent.SetVisibility` (`self.TextRender`) false true)
  (`SceneComponent.SetHiddenInGame` (`self.StaticMesh`) true true)
  (`self.SetActorTickEnabled` false))

(event `self.ReceiveTick`
  (params (DeltaSeconds :type "Float (single-precision)"))
  (bind _my_camera_comp (`self.My Camera Comp`))
  (if (`self.overlapitem`)
    (`/Engine/EditorBlueprintResources/StandardMacros.IsValid` _my_camera_comp
      (:`Is Valid`
        (`SceneComponent.K2_SetWorldRotation` (`self.TextRender`) (`KismetMathLibrary.FindLookAtRotation` (`SceneComponent.K2_GetComponentLocation` (`self.TextRender`)) (`SceneComponent.K2_GetComponentLocation` _my_camera_comp)) false false)))))

(fn `UserConstructionScript`)