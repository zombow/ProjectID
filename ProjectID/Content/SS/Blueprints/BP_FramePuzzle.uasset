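; Frame puzzle actor that reveals its picture meshes and opens a pair of curtains when the puzzle is solved.
; FramePuzzleSolved shows the meshes, then CurtainOpen lerps each referenced curtain's X scale toward its open value using delta seconds, so repeated calls ease the motion.
; A DoOnce limits the frame-placing sound and both attenuated curtain sounds to the first call.
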(event `self.ReceiveBeginPlay`
  (`self.EnableInput` (`GameplayStatics.GetPlayerController` 0)))

(event `self.ReceiveTick`
  (params (DeltaSeconds :type "Float (single-precision)")))

(event `/Game/DY/Blueprints/BPI_ItemInteraction.FramePuzzleSolved`
  (bind _returnvalue (`GameplayStatics.GetWorldDeltaSeconds`))
  (`SceneComponent.SetVisibility` (`self.StaticMesh`) true false)
  (`SceneComponent.SetVisibility` (`self.Plane`) true false)
  (`|ExecutionSequence`
    (:`then_0`
      (`self.CurtainOpen` _returnvalue _returnvalue))
    (:`then_1`
      (`/Engine/EditorBlueprintResources/StandardMacros.DoOnce` false
        (:`Completed`
          (`GameplayStatics.PlaySoundAtLocation` "/Game/CYS/CYS_Sound/아이템놓는소리/액자_놓는_소리.액자_놓는_소리" (`SceneComponent.K2_GetComponentLocation` (`self.StaticMesh`)) (struct) 1.0 1.0 0.0 null null null null)
          (`GameplayStatics.PlaySoundAtLocation` "/Game/SS/Sound/CurtainSound.CurtainSound" (`self.K2_GetActorLocation` (`self.leftCurtain`)) (struct) 1.0 1.0 0.0 "/Game/SS/Sound/SA_clock.SA_clock" null null null)
          (`GameplayStatics.PlaySoundAtLocation` "/Game/SS/Sound/CurtainSound.CurtainSound" (`self.K2_GetActorLocation` (`self.rightCurtain`)) (struct) 1.0 1.0 0.0 "/Game/SS/Sound/SA_clock.SA_clock" null null null))))))

(fn `CurtainOpen`
  (params (Alpha :type "Float (double-precision)") (Alpha2 :type "Float (double-precision)"))
  (bind _leftcurtain (`self.leftCurtain`))
  (bind _rightcurtain (`self.rightCurtain`))
  (bind (_returnvalue_x _returnvalue_y _returnvalue_z) (`KismetMathLibrary.BreakVector` (`self.GetActorScale3D` _rightcurtain)))
  (bind (_returnvalue_x_2 _returnvalue_y_2 _returnvalue_z_2) (`KismetMathLibrary.BreakVector` (`self.GetActorScale3D` _leftcurtain)))
  (`self.SetActorScale3D` _leftcurtain (`KismetMathLibrary.MakeVector` (`KismetMathLibrary.Lerp` _returnvalue_x_2 1.0 Alpha) _returnvalue_y_2 _returnvalue_z_2))
  (`self.SetActorScale3D` _rightcurtain (`KismetMathLibrary.MakeVector` (`KismetMathLibrary.Lerp` _returnvalue_x -1.0 Alpha2) _returnvalue_y _returnvalue_z)))

(fn `UserConstructionScript`)