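; Directional combination padlock puzzle that opens a cabinet and enables pill and alcohol bottle collision when solved.
; Four directional inputs nudge the stick and record a code; Tick checks seven entries against CorrectCombination, clearing wrong attempts after a brief lockout.
; On success, Tick hides the lock, lerps both doors open and calls the player's UnlockMessage.
; The player's DirLockOn flag toggles the interaction widget, mesh and camera-facing text.
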(event `self.ReceiveBeginPlay`
  (`|ExecutionSequence`
    (:`then_0`
      (bind _returnvalue (`|CreateWidget` "/Game/CYS/CYS_BluePrints/WBP_Interaction.WBP_Interaction_C"))
      (bind _output_get (set `self.interActionUI` _returnvalue))
      (`UserWidget.AddToViewport` _output_get 0)
      (`Widget.SetVisibility` _output_get "Collapsed"))
    (:`then_1`
      (`self.EnableInput` (`GameplayStatics.GetPlayerController` 0)))))

(event `self.ReceiveTick`
  (params (DeltaSeconds :type "Float (single-precision)"))
  (bind _returnvalue (`GameplayStatics.GetWorldDeltaSeconds`))
  (bind _interactionui (`self.interActionUI`))
  (bind _staticmesh (`self.StaticMesh`))
  (bind _cabinetdoorr (`self.CabinetDoorR`))
  (bind _cabinetdoorl (`self.CabinetDoorL`))
  (bind _my_camera_comp (`self.My Camera Comp`))
  (bind _textrender (`self.TextRender`))
  (bind (_returnvalue_roll _returnvalue_pitch _returnvalue_yaw) (`KismetMathLibrary.BreakRotator` (`self.K2_GetActorRotation` _cabinetdoorr)))
  (bind (_returnvalue_roll_2 _returnvalue_pitch_2 _returnvalue_yaw_2) (`KismetMathLibrary.BreakRotator` (`self.K2_GetActorRotation` _cabinetdoorl)))
  (`|ExecutionSequence`
    (:`then_0`
      (if (== (`KismetArrayLibrary.Array_Length` (`self.inputCombination`)) 7)
        (set `self.bCanNotInput` true)
        (for (_array_element _array_index) (`self.inputCombination`)
          (if (not (== (`|GetArrayItem` (`self.correctCombination`) _array_index) _array_element))
            (`/Engine/EditorBlueprintResources/StandardMacros.IncrementInt` (`self.failCaseNum`))))
        (if (> (`self.failCaseNum`) 0)
          (`KismetArrayLibrary.Array_Clear` (`self.inputCombination`))
          (set `self.failCaseNum` 0)
          (`KismetSystemLibrary.Delay` 1.0)
          (set `self.bCanNotInput` false)
          (else
            (`KismetArrayLibrary.Array_Clear` (`self.inputCombination`))
            (set `self.bSolved` true)
            (bind _returnvalue_2 (`GameplayStatics.GetActorOfClass` "/Game/DY/Blueprints/BP_PillBottle.BP_PillBottle_C"))
            (`/Game/DY/Blueprints/BP_PillBottle.Active Collision` _returnvalue_2)
            (bind _returnvalue_3 (`GameplayStatics.GetActorOfClass` "/Game/DY/Blueprints/BP_AlcoholBottle.BP_AlcoholBottle_C"))
            (`/Game/DY/Blueprints/BP_AlcoholBottle.Active Collision` _returnvalue_3)))))
    (:`then_1`
      (if (`self.bSolved`)
        (`SceneComponent.SetVisibility` (`self.Lockbody`) false false)
        (`SceneComponent.SetVisibility` (`self.DirStick`) false false)
        (`self.K2_SetActorRotation` _cabinetdoorr (`KismetMathLibrary.MakeRotator` 0.0 0.0 (`KismetMathLibrary.Lerp` _returnvalue_yaw -120.0 _returnvalue)) false)
        (`self.K2_SetActorRotation` _cabinetdoorl (`KismetMathLibrary.MakeRotator` 0.0 0.0 (`KismetMathLibrary.Lerp` _returnvalue_yaw_2 120.0 _returnvalue)) false)
        (`KismetSystemLibrary.Delay` 1.0)
        (message `/Game/DY/Blueprints/BPI_ItemInteraction.Unlock` (`GameplayStatics.GetPlayerCharacter` 0))))
    (:`then_2`
      ;[1 0.9065 0.7728 1 48] 오버랩 인식
      (bind _asayu_test_character (cast `/Game/AYU/AYU_Blueprints/AYU_TestCharacter` (`GameplayStatics.GetPlayerCharacter` 0)))
      (bind _output_get (set `self.Dir Lock On` (`/Game/AYU/AYU_Blueprints/AYU_TestCharacter.Dir Lock On` _asayu_test_character)))
      (set `self.My Camera Comp` (`TestCharacter.myCameraComp` _asayu_test_character))
      (if _output_get
        (set `self.overlapitem` true)
        (`Widget.SetVisibility` _interactionui "HitTestInvisible")
        (`SceneComponent.SetVisibility` _textrender true true)
        (`SceneComponent.SetHiddenInGame` _staticmesh false true)
        ;[1 1 1 1 42] 3D텍스트회전
        (if (`self.overlapitem`)
          (`/Engine/EditorBlueprintResources/StandardMacros.IsValid` _my_camera_comp
            (:`Is Valid`
              (`SceneComponent.K2_SetWorldRotation` (`self.TextRender`) (`KismetMathLibrary.FindLookAtRotation` (`SceneComponent.K2_GetComponentLocation` (`self.TextRender`)) (`SceneComponent.K2_GetComponentLocation` _my_camera_comp)) false false))))
        (else
          (set `self.overlapitem` false)
          (`Widget.SetVisibility` _interactionui "Hidden")
          (`SceneComponent.SetVisibility` _textrender false true)
          (`SceneComponent.SetHiddenInGame` _staticmesh true true))))))

(event `InputAction|UpLockMove`
  (params (Key :type "Key Structure"))
  (bind _dirstick (`self.DirStick`))
  (bind _dirstick_2 (`self.DirStick`))
  (bind (_relativelocation_x _relativelocation_y _relativelocation_z) (`KismetMathLibrary.BreakVector` (`SceneComponent.RelativeLocation` _dirstick_2)))
  (bind (_relativelocation_x_2 _relativelocation_y_2 _relativelocation_z_2) (`KismetMathLibrary.BreakVector` (`SceneComponent.RelativeLocation` _dirstick)))
  (:`Pressed`
    (`GameplayStatics.PlaySound2D` "/Game/CYS/CYS_Sound/CYS_SFX/자물쇠_키입력.자물쇠_키입력" 1.0 1.0 0.0 null null)
    (if (not (`self.bCanNotInput`))
      (set `self.bCanNotInput` true)
      (`SceneComponent.K2_SetRelativeLocation` _dirstick_2 (`KismetMathLibrary.MakeVector` 0.5 _relativelocation_y _relativelocation_z) false false)
      (`KismetSystemLibrary.Delay` 0.2)
      (`SceneComponent.K2_SetRelativeLocation` _dirstick (`KismetMathLibrary.MakeVector` 0.0 _relativelocation_y_2 _relativelocation_z_2) false false)
      (`KismetArrayLibrary.Array_Add` (`self.inputCombination`) 1)
      (set `self.bCanNotInput` false))))

(event `InputAction|DownLockMove`
  (params (Key :type "Key Structure"))
  (bind _dirstick (`self.DirStick`))
  (bind _dirstick_2 (`self.DirStick`))
  (bind (_relativelocation_x _relativelocation_y _relativelocation_z) (`KismetMathLibrary.BreakVector` (`SceneComponent.RelativeLocation` _dirstick)))
  (bind (_relativelocation_x_2 _relativelocation_y_2 _relativelocation_z_2) (`KismetMathLibrary.BreakVector` (`SceneComponent.RelativeLocation` _dirstick_2)))
  (:`Pressed`
    (`GameplayStatics.PlaySound2D` "/Game/CYS/CYS_Sound/CYS_SFX/자물쇠_키입력.자물쇠_키입력" 1.0 1.0 0.0 null null)
    (if (not (`self.bCanNotInput`))
      (set `self.bCanNotInput` true)
      (`SceneComponent.K2_SetRelativeLocation` _dirstick_2 (`KismetMathLibrary.MakeVector` -0.5 _relativelocation_y_2 _relativelocation_z_2) false false)
      (`KismetSystemLibrary.Delay` 0.2)
      (`SceneComponent.K2_SetRelativeLocation` _dirstick (`KismetMathLibrary.MakeVector` 0.0 _relativelocation_y _relativelocation_z) false false)
      (`KismetArrayLibrary.Array_Add` (`self.inputCombination`) 3)
      (set `self.bCanNotInput` false))))

(event `InputAction|RightLockMove`
  (params (Key :type "Key Structure"))
  (bind _dirstick (`self.DirStick`))
  (bind _dirstick_2 (`self.DirStick`))
  (bind (_relativelocation_x _relativelocation_y _relativelocation_z) (`KismetMathLibrary.BreakVector` (`SceneComponent.RelativeLocation` _dirstick)))
  (bind (_relativelocation_x_2 _relativelocation_y_2 _relativelocation_z_2) (`KismetMathLibrary.BreakVector` (`SceneComponent.RelativeLocation` _dirstick_2)))
  (:`Pressed`
    (`GameplayStatics.PlaySound2D` "/Game/CYS/CYS_Sound/CYS_SFX/자물쇠_키입력.자물쇠_키입력" 1.0 1.0 0.0 null null)
    (if (not (`self.bCanNotInput`))
      (set `self.bCanNotInput` true)
      (`SceneComponent.K2_SetRelativeLocation` _dirstick (`KismetMathLibrary.MakeVector` _relativelocation_x 0.5 _relativelocation_z) false false)
      (`KismetSystemLibrary.Delay` 0.2)
      (`SceneComponent.K2_SetRelativeLocation` _dirstick_2 (`KismetMathLibrary.MakeVector` _relativelocation_x_2 0.0 _relativelocation_z_2) false false)
      (`KismetArrayLibrary.Array_Add` (`self.inputCombination`) 2)
      (set `self.bCanNotInput` false))))

(event `InputAction|LeftLockMove`
  (params (Key :type "Key Structure"))
  (bind _dirstick (`self.DirStick`))
  (bind _dirstick_2 (`self.DirStick`))
  (bind (_relativelocation_x _relativelocation_y _relativelocation_z) (`KismetMathLibrary.BreakVector` (`SceneComponent.RelativeLocation` _dirstick_2)))
  (bind (_relativelocation_x_2 _relativelocation_y_2 _relativelocation_z_2) (`KismetMathLibrary.BreakVector` (`SceneComponent.RelativeLocation` _dirstick)))
  (:`Pressed`
    (`GameplayStatics.PlaySound2D` "/Game/CYS/CYS_Sound/CYS_SFX/자물쇠_키입력.자물쇠_키입력" 1.0 1.0 0.0 null null)
    (if (not (`self.bCanNotInput`))
      (set `self.bCanNotInput` true)
      (`SceneComponent.K2_SetRelativeLocation` _dirstick_2 (`KismetMathLibrary.MakeVector` _relativelocation_x -0.5 _relativelocation_z) false false)
      (`KismetSystemLibrary.Delay` 0.2)
      (`SceneComponent.K2_SetRelativeLocation` _dirstick (`KismetMathLibrary.MakeVector` _relativelocation_x_2 0.0 _relativelocation_z_2) false false)
      (`KismetArrayLibrary.Array_Add` (`self.inputCombination`) 4)
      (set `self.bCanNotInput` false))))

(fn `UserConstructionScript`)