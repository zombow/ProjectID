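; BP_Diary is an inspectable diary item that shows a diary page widget with narration.
; On BeginPlay it runs the parent logic, then creates a WBP_DiaryPage and adds it to the viewport.
; CheckItem with ViewProps true reveals the page, plays a book sound and spawns a BP_Naration actor carrying six diary dialogue entries.
; With ViewProps false it hides the page and destroys that narration actor.
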(event `self.ReceiveBeginPlay`
  (`parent.ReceiveBeginPlay`)
  (`|ExecutionSequence`
    (:`then_0`
      (bind _returnvalue (`|CreateWidget` "/Game/DY/Blueprints/WBP_DiaryPage.WBP_DiaryPage_C"))
      (bind _output_get (set `self.UI` _returnvalue))
      (`UserWidget.AddToViewport` _output_get 0))))

(event `/Game/DY/Blueprints/BPI_ItemInteraction.CheckItem`
  (params (viewProps :type Boolean))
  (bind _ui (`self.UI`))
  (if viewProps
    (`Widget.SetVisibility` _ui "SelfHitTestInvisible")
    (`GameplayStatics.SpawnSound2D` "/Game/CYS/CYS_Sound/아이템먹는소리/책5.책5" 1.0 1.0 0.0 null)
    (bind _returnvalue (`|SpawnActorFromClass` "/Game/CYS/CYS_Voice/BP_Naration.BP_Naration_C" (`SceneComponent.K2_GetComponentToWorld` (`self.DefaultSceneRoot`)) "AlwaysSpawn" "OverrideRootScale" null "/Game/CYS/CYS_Voice/Diary_Naration/DiaryNaration_1.DiaryNaration_1" "/Game/CYS/CYS_Voice/Diary_Naration/DiaryNaration_2.DiaryNaration_2" "/Game/CYS/CYS_Voice/Diary_Naration/DiaryNaration_6.DiaryNaration_6" "/Game/CYS/CYS_Voice/Diary_Naration/DiaryNaration_4.DiaryNaration_4" "/Game/CYS/CYS_Voice/Diary_Naration/DiaryNaration_5.DiaryNaration_5" "/Game/CYS/CYS_Voice/Diary_Naration/DiaryNaration_3.DiaryNaration_3" null))
    (else
      (`Widget.SetVisibility` _ui "Hidden")
      (`self.K2_DestroyActor` _returnvalue))))

(fn `UserConstructionScript`)