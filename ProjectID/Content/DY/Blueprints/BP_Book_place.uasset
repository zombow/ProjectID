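; BP_Book_place is an inspectable book actor that shows or hides a full-screen book widget when checked.
; On BeginPlay it runs the parent logic, then creates WBP_Book_place and adds it to the viewport.
; CheckItem toggles that widget's visibility with a matching 2D sound for opening or putting down.
; Opening also sets IsChecked and sends interaction message 0 to the level's BP_WorldLightCtrl.
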(event `self.ReceiveBeginPlay`
  (`parent.ReceiveBeginPlay`)
  (bind _returnvalue (`|CreateWidget` "/Game/DY/Blueprints/WBP_Book_place.WBP_Book_place_C"))
  (bind _output_get (set `self.UI` _returnvalue))
  (`UserWidget.AddToViewport` _output_get 0))

(event `/Game/DY/Blueprints/BPI_ItemInteraction.CheckItem`
  (params (viewProps :type Boolean))
  (bind _ui (`self.UI`))
  (if viewProps
    (`Widget.SetVisibility` _ui "SelfHitTestInvisible")
    (`GameplayStatics.SpawnSound2D` "/Game/CYS/CYS_Sound/아이템먹는소리/책3.책3" 1.0 1.0 0.0 null)
    (set `self.bIsChecked` true)
    (bind _returnvalue (`GameplayStatics.GetActorOfClass` "/Game/SS/Blueprints/BP_WorldLightCtrl.BP_WorldLightCtrl_C"))
    (message `LevelInterface.ProccedInteraction` _returnvalue 0)
    (else
      (`Widget.SetVisibility` _ui "Hidden")
      (`GameplayStatics.SpawnSound2D` "/Game/CYS/CYS_Sound/아이템놓는소리/물건_놓는_소리_2.물건_놓는_소리_2" 1.0 1.0 0.0 null))))

(fn `UserConstructionScript`)