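; BP_SafeBox is a safe that opens its door and activates collision on the level's BP_Ring.
; SafeOpen runs once, playing a key sound, then two seconds later setting an open flag and replacing its tags.
; While open, Tick lerps the door toward a fixed world rotation and disables the box collision.
; When the key sound finishes, a door sound plays and the ring's collision activates.
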(event `self.ReceiveBeginPlay`
  (bind _returnvalue (`GameplayStatics.GetActorOfClass` "/Game/DY/Blueprints/BP_Ring.BP_Ring_C"))
  (set `self.Ring` _returnvalue))

(event `self.ReceiveTick`
  (params (DeltaSeconds :type "Float (single-precision)"))
  (if (`self.beOpen`)
    (`SceneComponent.K2_SetWorldRotation` (`self.SafeDoor`) (`KismetMathLibrary.RLerp` (`SceneComponent.K2_GetComponentRotation` (`self.SafeDoor`)) (struct :`Yaw` 30.0) DeltaSeconds) false false)
    (`PrimitiveComponent.SetCollisionEnabled` (`self.Box`) "NoCollision")))

(event `self.Box.OnComponentBeginOverlap`
  (params (OverlappedComponent :type "PrimitiveComponent Object Reference") (OtherActor :type "Actor Object Reference") (OtherComp :type "PrimitiveComponent Object Reference") (OtherBodyIndex :type Integer) (bFromSweep :type Boolean) (SweepResult :type "HitResult Structure (by ref)"))
  (cast `TestCharacter` OtherActor)
  (if (`self.beKeyClicked`)
    _))

(event `/Game/DY/Blueprints/BPI_ItemInteraction.SafeOpen`
  (params (bIsKeyClicked :type Boolean))
  (`/Engine/EditorBlueprintResources/StandardMacros.DoOnce` false
    (:`Completed`
      (bind _returnvalue (`GameplayStatics.SpawnSoundAtLocation` "/Game/SoundFile/KeyOpenSound.KeyOpenSound" (`SceneComponent.K2_GetComponentLocation` (`self.SafeDoor`)) (struct) 1.0 1.0 0.0 null null))
      (`|ExecutionSequence`
        (:`then_0`
          (`KismetSystemLibrary.Delay` 2.0)
          (set `self.beOpen` true)
          (set `self.Tags` (`self.Tags_0`)))
        (:`then_1`
          (add `AudioComponent.OnAudioFinished` _returnvalue (delegate `OpenSoundplay`)))))))

(event `OpenSoundplay`
  (`GameplayStatics.PlaySoundAtLocation` "/Game/CYS/CYS_Sound/CYS_SFX/금고문여는소리.금고문여는소리" (`SceneComponent.K2_GetComponentLocation` (`self.SafeDoor`)) (struct) 1.0 1.0 0.0 null null null null)
  (`KismetSystemLibrary.PrintString` "Hello")
  (`/Game/DY/Blueprints/BP_Ring.Active Collision` (`self.Ring`)))

(fn `UserConstructionScript`)