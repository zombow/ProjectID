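; BP_Book_in is a book item actor that shows a UI widget when it is checked.
; On BeginPlay it runs the parent logic, then creates and stores a WBP_Book_in widget.
; CheckItem adds that widget to the viewport, sets IsChecked and sends interaction message 0 to an actor found by class, or removes the widget when ViewProps is false.
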(event `self.ReceiveBeginPlay`
  (`parent.ReceiveBeginPlay`)
  (bind _returnvalue (`|CreateWidget` "/Game/DY/Blueprints/WBP_Book_in.WBP_Book_in_C"))
  (set `self.UI` _returnvalue))

(event `/Game/DY/Blueprints/BPI_ItemInteraction.CheckItem`
  (params (viewProps :type Boolean))
  (bind _ui (`self.UI`))
  (if viewProps
    (`UserWidget.AddToViewport` _ui 0)
    (set `self.bIsChecked` true)
    (bind _returnvalue (`GameplayStatics.GetActorOfClass` null))
    (message `LevelInterface.ProccedInteraction` _returnvalue 0)
    (else
      (`Widget.RemoveFromParent` _ui))))

(fn `UserConstructionScript`)